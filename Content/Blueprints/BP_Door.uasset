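; BP_Door is a door Blueprint that moves vertically when opened or closed by a button.
; On BeginPlay it finds a BP_Button via GetActorOfClass and binds OpenDoor and CloseDoor to that button's open and close events.
; Each event uses MoveComponentTo to shift the static mesh up or down by a fixed offset, adding it to the current world location but passing the result as a relative target.
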(event `self.ReceiveBeginPlay`
  (bind _returnvalue (`GameplayStatics.GetActorOfClass` "/Game/Blueprints/BP_Button.BP_Button_C"))
  (bind _output_get (set `self.Button Ref` _returnvalue))
  (add `/Game/Blueprints/BP_Button.Open` _output_get (delegate `Open Door`))
  (add `/Game/Blueprints/BP_Button.Close` _output_get (delegate `Close Door`)))

(event `Open Door`
  (bind _staticmeshcomponent (`self.StaticMeshComponent`))
  (`KismetSystemLibrary.MoveComponentTo` _staticmeshcomponent (+ (`SceneComponent.K2_GetComponentLocation` _staticmeshcomponent) (0.0 0.0 300.0))))

(event `Close Door`
  (bind _staticmeshcomponent (`self.StaticMeshComponent`))
  (`KismetSystemLibrary.MoveComponentTo` _staticmeshcomponent (+ (`SceneComponent.K2_GetComponentLocation` _staticmeshcomponent) (0.0 0.0 -300.0))))

(fn `UserConstructionScript`)