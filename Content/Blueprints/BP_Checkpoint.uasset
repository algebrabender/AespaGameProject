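; One-shot checkpoint actor that saves progress to slot "save1" when its Box is overlapped, then destroys itself.
; On overlap it sets UseSavedLocation, records itself in CheckpointsUsed, writes the slot, then calls SaveGame on BP_ThirdPersonGameMode.
; On BeginPlay it destroys itself if the existing save already lists it as used.
; Overlap does not filter the overlapping actor and stops if no BP_SaveGame loads.
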(event `self.ReceiveBeginPlay`
  (bind _returnvalue (`GameplayStatics.DoesSaveGameExist` "save1"))
  (if _returnvalue
    (bind _returnvalue_2 (`GameplayStatics.LoadGameFromSlot` "save1"))
    (bind _asbp_save_game (cast `/Game/Blueprints/BP_SaveGame` _returnvalue_2))
    (if (`KismetArrayLibrary.Array_Contains` (`/Game/Blueprints/BP_SaveGame.CheckpointsUsed` _asbp_save_game) self)
      (`self.K2_DestroyActor`))))

(event `self.Box.OnComponentBeginOverlap`
  (params (OverlappedComponent :type "PrimitiveComponent Object Reference") (OtherActor :type "Actor Object Reference") (OtherComp :type "PrimitiveComponent Object Reference") (OtherBodyIndex :type Integer) (bFromSweep :type Boolean) (SweepResult :type "HitResult Structure (by ref)"))
  (bind _returnvalue (`GameplayStatics.LoadGameFromSlot` "save1"))
  (bind _asbp_save_game (cast `/Game/Blueprints/BP_SaveGame` _returnvalue))
  (set `/Game/Blueprints/BP_SaveGame.UseSavedLocation` true _asbp_save_game)
  (`KismetArrayLibrary.Array_Add` (`/Game/Blueprints/BP_SaveGame.CheckpointsUsed` _asbp_save_game) self)
  (`GameplayStatics.SaveGameToSlot` _asbp_save_game "save1")
  (bind _asbp_third_person_game_mode (cast `/Game/ThirdPerson/Blueprints/BP_ThirdPersonGameMode` (`GameplayStatics.GetGameMode`)))
  (`/Game/ThirdPerson/Blueprints/BP_ThirdPersonGameMode.Save Game` _asbp_third_person_game_mode)
  (`self.K2_DestroyActor`))

(fn `UserConstructionScript`)