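; Health pickup actor that restores 20 health to the third-person character on overlap.
; On BeginPlay it sets the cube's material from a symbol material array, indexed by the character index stored in the game instance.
; The box overlap only heals when health is at most 80, then updates the character's health bar and destroys the pickup.
; Tick slowly spins the cube as a visual cue.
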(event `self.ReceiveBeginPlay`
  (bind _asgame_instance_blueprint (cast `/Game/Blueprints/GameInstanceBlueprint` (`GameplayStatics.GetGameInstance`)))
  (`PrimitiveComponent.SetMaterial` (`self.Cube`) 0 (`|GetArrayItem` (`self.SymbolMatArray`) (`/Game/Blueprints/GameInstanceBlueprint.CharacterIndex` _asgame_instance_blueprint))))

(event `self.Box.OnComponentBeginOverlap`
  (params (OverlappedComponent :type "PrimitiveComponent Object Reference") (OtherActor :type "Actor Object Reference") (OtherComp :type "PrimitiveComponent Object Reference") (OtherBodyIndex :type Integer) (bFromSweep :type Boolean) (SweepResult :type "HitResult Structure (by ref)"))
  (bind _asbp_third_person_character (cast `/Game/ThirdPerson/Blueprints/BP_ThirdPersonCharacter` OtherActor))
  (bind _health (`/Game/ThirdPerson/Blueprints/BP_ThirdPersonCharacter.Health` _asbp_third_person_character))
  (if (<= _health 80.0)
    (bind _output_get (set `/Game/ThirdPerson/Blueprints/BP_ThirdPersonCharacter.Health` (+ _health 20.0) _asbp_third_person_character))
    (`/Game/UI/Widgets/HealthWidgetBlueprint.UpdateHealthBar` (`/Game/ThirdPerson/Blueprints/BP_ThirdPersonCharacter.HealthBar` _asbp_third_person_character) _output_get)
    (`self.K2_DestroyActor`)))

(event `self.ReceiveTick`
  (params (DeltaSeconds :type "Float (single-precision)"))
  (`SceneComponent.K2_AddWorldRotation` (`self.Cube`) (struct :`Yaw` 1.0) false false))

(fn `UserConstructionScript`)