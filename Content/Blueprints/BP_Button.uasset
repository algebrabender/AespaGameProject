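; BP_Button is a pressure button that signals open and close as something enters and leaves its sphere trigger.
; Begin overlap fires the Open dispatcher and moves the mesh down; end overlap fires Close and moves it up.
; Both MoveComponentTo calls compute the target from the mesh's world location plus a vertical offset, though the input expects a relative location.
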(event `self.Sphere.OnComponentBeginOverlap`
  (params (OverlappedComponent :type "PrimitiveComponent Object Reference") (OtherActor :type "Actor Object Reference") (OtherComp :type "PrimitiveComponent Object Reference") (OtherBodyIndex :type Integer) (bFromSweep :type Boolean) (SweepResult :type "HitResult Structure (by ref)"))
  (bind _staticmeshcomponent (`self.StaticMeshComponent`))
  (`self.Open`)
  (`KismetSystemLibrary.MoveComponentTo` _staticmeshcomponent (+ (`SceneComponent.K2_GetComponentLocation` _staticmeshcomponent) (0.0 0.0 -10.0))))

(event `self.Sphere.OnComponentEndOverlap`
  (params (OverlappedComponent :type "PrimitiveComponent Object Reference") (OtherActor :type "Actor Object Reference") (OtherComp :type "PrimitiveComponent Object Reference") (OtherBodyIndex :type Integer))
  (bind _staticmeshcomponent (`self.StaticMeshComponent`))
  (`self.Close`)
  (`KismetSystemLibrary.MoveComponentTo` _staticmeshcomponent (+ (`SceneComponent.K2_GetComponentLocation` _staticmeshcomponent) (0.0 0.0 10.0))))

(fn `UserConstructionScript`)