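; BP_HealthItem is a spinning health pickup that adds 20 HP to BP_ThirdPersonCharacter and destroys itself.
; On BeginPlay it sets its cube material by the game instance's character index, then removes itself if its actor-and-transform struct is in the "save1" slot's HealthItemsUsed.
; Any box overlap adds that struct to a freshly loaded save object before the character check, but this Blueprint never writes it back to the slot.
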(event `self.ReceiveBeginPlay`
  (bind _asbp_game_inst (cast `/Game/Blueprints/BP_GameInst` (`GameplayStatics.GetGameInstance`)))
  (`PrimitiveComponent.SetMaterial` (`self.Cube`) 0 (`|GetArrayItem` (`self.SymbolMatArray`) (`/Game/Blueprints/BP_GameInst.CharacterIndex` _asbp_game_inst)))
  (bind _returnvalue (`GameplayStatics.LoadGameFromSlot` "save1"))
  (bind _asbp_save_game (cast `/Game/Blueprints/BP_SaveGame` _returnvalue))
  (if (`KismetArrayLibrary.Array_Contains` (`/Game/Blueprints/BP_SaveGame.HealthItemsUsed` _asbp_save_game) (make `/Game/Structs/HealthItemSaveInfoStruct` self (`SceneComponent.K2_GetComponentToWorld` (`self.Box`))))
    (`self.K2_DestroyActor`)))

(event `self.Box.OnComponentBeginOverlap`
  (params (OverlappedComponent :type "PrimitiveComponent Object Reference") (OtherActor :type "Actor Object Reference") (OtherComp :type "PrimitiveComponent Object Reference") (OtherBodyIndex :type Integer) (bFromSweep :type Boolean) (SweepResult :type "HitResult Structure (by ref)"))
  (bind _returnvalue (`GameplayStatics.LoadGameFromSlot` "save1"))
  (bind _asbp_save_game (cast `/Game/Blueprints/BP_SaveGame` _returnvalue))
  (`KismetArrayLibrary.Array_Add` (`/Game/Blueprints/BP_SaveGame.HealthItemsUsed` _asbp_save_game) (make `/Game/Structs/HealthItemSaveInfoStruct` self (`SceneComponent.K2_GetComponentToWorld` (`self.Box`))))
  (bind _asbp_third_person_character (cast `/Game/ThirdPerson/Blueprints/BP_ThirdPersonCharacter` OtherActor))
  (if true
    (set `/Game/ThirdPerson/Blueprints/BP_ThirdPersonCharacter.HP` (+ (`/Game/ThirdPerson/Blueprints/BP_ThirdPersonCharacter.HP` _asbp_third_person_character) 20) _asbp_third_person_character)
    (`self.K2_DestroyActor`)))

(event `self.ReceiveTick`
  (params (DeltaSeconds :type "Float (single-precision)"))
  (`SceneComponent.K2_AddWorldRotation` (`self.Cube`) (struct :`Yaw` 1.0) false false))

(fn `UserConstructionScript`)