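; Game mode Blueprint that handles saving, restarting and level-change bookkeeping through BP_SaveGame.
; SaveGame copies the player's transform, stats and character index into the save object, reading slot "save4" but writing "save1".
; LoadGame only restarts the level, while RestartLevel also deletes "save1" first.
; ChangeLevels clears the saved-location flag in "save1" without travelling to another level.
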(event `Save Game`
  (bind _asbp_third_person_character (cast `/Game/ThirdPerson/Blueprints/BP_ThirdPersonCharacter` (`GameplayStatics.GetPlayerCharacter` 0) :!pure true))
  ;[1 1 1] Save Game
  (bind _returnvalue (`GameplayStatics.LoadGameFromSlot` "save4"))
  (bind _asbp_save_game (cast `/Game/Blueprints/BP_SaveGame` _returnvalue))
  (set `/Game/Blueprints/BP_SaveGame.CharTransform` (`self.GetTransform` _asbp_third_person_character) _asbp_save_game)
  (set `/Game/Blueprints/BP_SaveGame.UseSavedLocation` true _asbp_save_game)
  (set `/Game/Blueprints/BP_SaveGame.CurrentLevel` (`/Game/ThirdPerson/Blueprints/BP_ThirdPersonCharacter.Level` _asbp_third_person_character) _asbp_save_game)
  (set `/Game/Blueprints/BP_SaveGame.CurrentHP` (`/Game/ThirdPerson/Blueprints/BP_ThirdPersonCharacter.HP` _asbp_third_person_character) _asbp_save_game)
  (set `/Game/Blueprints/BP_SaveGame.CurrentMaxHP` (`/Game/ThirdPerson/Blueprints/BP_ThirdPersonCharacter.LevelMaxHP` _asbp_third_person_character) _asbp_save_game)
  (set `/Game/Blueprints/BP_SaveGame.CurrentXP` (`/Game/ThirdPerson/Blueprints/BP_ThirdPersonCharacter.XP` _asbp_third_person_character) _asbp_save_game)
  (set `/Game/Blueprints/BP_SaveGame.CurrentMaxXP` (`/Game/ThirdPerson/Blueprints/BP_ThirdPersonCharacter.LevelMaxXP` _asbp_third_person_character) _asbp_save_game)
  (set `/Game/Blueprints/BP_SaveGame.CharacterIndex` (`/Game/Blueprints/BP_GameInst.CharacterIndex` (cast `/Game/Blueprints/BP_GameInst` (`GameplayStatics.GetGameInstance`) :!pure true)) _asbp_save_game)
  (`GameplayStatics.SaveGameToSlot` _asbp_save_game "save1"))

(event `Load Game`
  ;[1 1 1] Load Game
  (`KismetSystemLibrary.ExecuteConsoleCommand` "RestartLevel" null))

(event `Restart Level`
  ;[1 1 1] Restart Level
  (`GameplayStatics.DeleteGameInSlot` "save1")
  (`KismetSystemLibrary.ExecuteConsoleCommand` "RestartLevel" null))

(event `ChangeLevels`
  ;[1 1 1] Change Levels
  (bind _returnvalue (`GameplayStatics.LoadGameFromSlot` "save1"))
  (bind _asbp_save_game (cast `/Game/Blueprints/BP_SaveGame` _returnvalue))
  (set `/Game/Blueprints/BP_SaveGame.UseSavedLocation` false _asbp_save_game)
  (`GameplayStatics.SaveGameToSlot` _asbp_save_game "save1"))

(fn `UserConstructionScript`)